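; GoToNextLevel is a level-exit trigger that loads the next numbered level when the player reaches its sphere.
; The sphere is made visible on BeginPlay and reacts only to overlapping actors whose display name is "PlayerStart".
; It builds the next level name from the current name's first five characters plus the following single digit incremented, prints it, then opens that level.
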(event `self.ReceiveBeginPlay`
  (`SceneComponent.SetHiddenInGame` (`self.Sphere`) false false))

(event `self.Sphere.OnComponentBeginOverlap`
  (params (OverlappedComponent :type "PrimitiveComponent Object Reference") (OtherActor :type "Actor Object Reference") (OtherComp :type "PrimitiveComponent Object Reference") (OtherBodyIndex :type Integer) (bFromSweep :type Boolean) (SweepResult :type "HitResult Structure (by ref)"))
  (if (`KismetStringLibrary.EqualEqual_StrStr` (`KismetSystemLibrary.GetDisplayName` OtherActor) "PlayerStart")
    (bind _returnvalue (`GameplayStatics.GetCurrentLevelName` true))
    (bind _returnvalue_2 (`KismetStringLibrary.Concat_StrStr` (`KismetStringLibrary.Left` _returnvalue 5) (`KismetStringLibrary.Conv_IntToString` (+ (`KismetStringLibrary.Conv_StringToInt` (`KismetStringLibrary.Mid` _returnvalue 5 1)) 1))))
    (`KismetSystemLibrary.PrintString` _returnvalue_2)
    (`GameplayStatics.OpenLevel` (`KismetStringLibrary.Conv_StringToName` _returnvalue_2))))

(fn `UserConstructionScript`)