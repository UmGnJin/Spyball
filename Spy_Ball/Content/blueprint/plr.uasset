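; Player pawn that moves by charge-and-release physics launches along the control rotation, limited by a jump charge count.
; Holding left click builds power in Tick, and release launches the mesh; charges refill when it rests on flat ground.
; Right click fires a double-power Super launch when available.
; The wheel-toggled Ninja skill freezes physics on hitting a different object than last time, sticking there and refilling charges.
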(event `self.ReceiveBeginPlay`
  (set `self.cur_skill_super` (`self.skill_super`))
  (set `self.cur_skill_ninja` (`self.skill_ninja`))
  (set `self.cur_charge_count` (`self.max_charge_count`)))

(event `self.ReceiveHit`
  (params (MyComp :type "PrimitiveComponent Object Reference") (Other :type "Actor Object Reference") (OtherComp :type "PrimitiveComponent Object Reference") (bSelfMoved :type Boolean) (HitLocation :type "Vector Structure") (HitNormal :type "Vector Structure") (NormalImpulse :type "Vector Structure") (Hit :type "HitResult Structure (by ref)"))
  (set `self.ninja_Z` (.z HitNormal))
  (if (and (!= Other (`self.ninja_previous_wall`)) (`self.cur_skill_ninja`))
    (set `self.ninja_previous_wall` Other)
    (set `self.ninja_anywhere` true)))

(event `self.ReceiveTick`
  (params (DeltaSeconds :type "Float (single-precision)"))
  (bind _plr_mesh (`self.plr_mesh`))
  (bind _charge_amount (`self.charge_amount`))
  (if (`self.charging`)
    (if (> 1.0 _charge_amount)
      (set `self.charge_amount` (+ _charge_amount DeltaSeconds)))
    (elif (> _charge_amount 0.0)
      (`PrimitiveComponent.SetSimulatePhysics` _plr_mesh true)
      (`PrimitiveComponent.SetAllPhysicsLinearVelocity` _plr_mesh (0.0 0.0 0.0) false)
      (`PrimitiveComponent.AddForce` _plr_mesh (* (`self.charge_direction`) (* _charge_amount (`self.super_charge`) 50000000.0)) "None" false)
      (set `self.charge_amount` 0.0)
      (set `self.cur_charge_count` (- (`self.cur_charge_count`) 1))
      (set `self.ninja_Z` 0.0)
      (set `self.ninja_anywhere` false)
      (set `self.super_charge` 1.0)
      (elif (and (> (`self.ninja_Z`) 0.9) (> 1.0 (`KismetMathLibrary.VSize` (`self.GetVelocity`))))
        (set `self.cur_charge_count` (`self.max_charge_count`) :!label _label)
        (if (`self.skill_super`)
          (set `self.cur_skill_super` true))
        (elif (`self.ninja_anywhere`)
          (`PrimitiveComponent.SetSimulatePhysics` (`self.plr_mesh`) false)
          (goto _label))))))

(event `InputAction|left_click`
  (params (Key :type "Key Structure"))
  (:`Pressed`
    (if (> (`self.cur_charge_count`) 0) :!label _label_2
      (set `self.charging` true)))
  (:`Released`
    (if (`self.charging`) :!label _label_3
      (set `self.charging` false)
      (set `self.charge_direction` (`KismetMathLibrary.Conv_RotatorToVector` (`self.GetControlRotation`))))))

(event `InputAction|right_click`
  (params (Key :type "Key Structure"))
  (bind _cur_skill_super (`self.cur_skill_super`))
  (:`Pressed`
    (if _cur_skill_super
      (set `self.super_charge` 2.0)
      (goto _label_2)))
  (:`Released`
    (if _cur_skill_super
      (set `self.cur_skill_super` false)
      (goto _label_3))))

(event `InputAxis|vertical_mouse`
  (params (AxisValue :type "Float (single-precision)"))
  (`self.AddControllerYawInput` AxisValue))

(event `InputAxis|horizontal_mouse`
  (params (AxisValue :type "Float (single-precision)"))
  (`self.AddControllerPitchInput` AxisValue))

(event `InputAction|upwheel_mouse`
  (params (Key :type "Key Structure"))
  (bind _cur_skill_ninja (`self.cur_skill_ninja`))
  (:`Pressed`
    (if (`self.skill_ninja`) :!label _label_4
      (set `self.cur_skill_ninja` (not _cur_skill_ninja))
      (`KismetSystemLibrary.PrintString` (`KismetStringLibrary.Concat_StrStr` "NINJA : " (`KismetStringLibrary.Conv_BoolToString` _cur_skill_ninja))))))

(event `InputAction|downwheel_mouse`
  (params (Key :type "Key Structure"))
  (:`Pressed`
    (goto _label_4)))

(fn `UserConstructionScript`)