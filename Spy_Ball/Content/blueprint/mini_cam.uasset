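; mini_cam is a possessable free-flying camera, tethered to the location where it was possessed.
; Mouse axes drive controller yaw and pitch, and three movement axes apply local offsets along control-rotation vectors without sweep or delta-time scaling.
; Tick recomputes NearLimit from squared distance to that start point, scaling movement in every direction down to zero at 1500 units.
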(event `self.ReceiveTick`
  (params (DeltaSeconds :type "Float (single-precision)"))
  (set `self.near_limit` (/ (- 2250000.0 (`KismetMathLibrary.Square` (`KismetMathLibrary.VSize` (- (`self.K2_GetActorLocation`) (`self.plr_location`))))) 2250000.0)))

(event `InputAxis|vertical_mouse`
  (params (AxisValue :type "Float (single-precision)"))
  (`self.AddControllerYawInput` AxisValue))

(event `InputAxis|horizontal_mouse`
  (params (AxisValue :type "Float (single-precision)"))
  (`self.AddControllerPitchInput` AxisValue))

(event `InputAxis|forward_back`
  (params (AxisValue :type "Float (single-precision)"))
  (`self.K2_AddActorLocalOffset` (* (* (`KismetMathLibrary.GetForwardVector` (`self.GetControlRotation`)) (* AxisValue (`self.near_limit`))) 5.0)))

(event `InputAxis|right_left`
  (params (AxisValue :type "Float (single-precision)"))
  (`self.K2_AddActorLocalOffset` (* (* (`KismetMathLibrary.GetRightVector` (`self.GetControlRotation`)) (* AxisValue (`self.near_limit`))) 5.0)))

(event `InputAxis|up_down`
  (params (AxisValue :type "Float (single-precision)"))
  (`self.K2_AddActorLocalOffset` (* (* (`KismetMathLibrary.GetUpVector` (`self.GetControlRotation`)) (* AxisValue (`self.near_limit`))) 5.0)))

(event `self.ReceivePossessed`
  (params (NewController :type "Controller Object Reference"))
  (set `self.plr_location` (`self.K2_GetActorLocation`))
  (set `self.near_limit` 1.0))

(fn `UserConstructionScript`)